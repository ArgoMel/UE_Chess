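; BattleChess player Blueprint that holds both players' state and controls the board camera.
; Player0 and Player1 structs track name, color, check and legal-move flags, move and capture counts, with lookups by index or color and setters that rebuild the struct.
; SetPlayerCamera eases the azimuth pivot back to zero while gliding the camera to the White or Black anchor transform.
; RotateCamera adds axis input to the pivot's yaw.
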(event Custom|SetPlayerCamera
  (params (PlayerColor :type EN_PlayerColor%20Enum :default "NewEnumerator0"))
  (bind _white (Variables|Default|GetWhite))
  (bind _black (Variables|Default|GetBlack))
  (bind _returnvalue (Transformation|GetRelativeTransform _black))
  (bind _returnvalue_2 (Transformation|GetRelativeTransform _white))
  (Components|MoveComponentTo (Variables|Default|GetCameraAzimuth) "0, 0, 0" "0, 0, 0" true true 1.0 true)
  (switch Utilities|FlowControl|Switch|SwitchonEN_PlayerColor PlayerColor
    (:NewEnumerator0
      (Components|MoveComponentTo (Variables|Default|GetCamera) (.location _returnvalue_2) (.rotation _returnvalue_2) true true 3.0 false))
    (:NewEnumerator1
      (Components|MoveComponentTo (Variables|Default|GetCamera) (.location _returnvalue) (.rotation _returnvalue) true true 3.0 false))))

(fn ConstructionScript)

(fn GetPlayerbyIndex
  (params (PlayerIndex :type Integer))
  (if (== PlayerIndex (.index (Variables|Default|GetPlayer0)))
    (return (Variables|Default|GetPlayer0))
    (else
      (return (Variables|Default|GetPlayer1)))))

(fn GetPlayerbyColor
  (params (PlayerColor :type EN_PlayerColor%20Enum :default "NewEnumerator0"))
  (if (Utilities|Enum|Equal(Enum) PlayerColor (.color (Variables|Default|GetPlayer0)))
    (return (Variables|Default|GetPlayer0))
    (else
      (return (Variables|Default|GetPlayer1)))))

(fn SetPlayerColor
  (params (PlayerIndex :type Integer) (PlayerColor :type EN_PlayerColor%20Enum :default "NewEnumerator0"))
  (switch int PlayerIndex
    (:0
      (Variables|Default|SetPlayer0 (Utilities|Struct|MakeST_Player (.Name (Utilities|Struct|BreakST_Player (Variables|Default|GetPlayer0))) PlayerColor (.Index (Utilities|Struct|BreakST_Player (Variables|Default|GetPlayer0))) (.isInCheckFlag (Utilities|Struct|BreakST_Player (Variables|Default|GetPlayer0))) (.HasLegalMoves (Utilities|Struct|BreakST_Player (Variables|Default|GetPlayer0))) (.MoveCount (Utilities|Struct|BreakST_Player (Variables|Default|GetPlayer0))) (.Captures (Utilities|Struct|BreakST_Player (Variables|Default|GetPlayer0))))))
    (:1
      (Variables|Default|SetPlayer1 (Utilities|Struct|MakeST_Player (.Name (Utilities|Struct|BreakST_Player (Variables|Default|GetPlayer1))) PlayerColor (.Index (Utilities|Struct|BreakST_Player (Variables|Default|GetPlayer1))) (.isInCheckFlag (Utilities|Struct|BreakST_Player (Variables|Default|GetPlayer1))) (.HasLegalMoves (Utilities|Struct|BreakST_Player (Variables|Default|GetPlayer1))) (.MoveCount (Utilities|Struct|BreakST_Player (Variables|Default|GetPlayer1))) (.Captures (Utilities|Struct|BreakST_Player (Variables|Default|GetPlayer1))))))))

(fn SetPlayerName
  (params (PlayerIndex :type Integer) (PlayerName :type String))
  (switch int PlayerIndex
    (:0
      (Variables|Default|SetPlayer0 (Utilities|Struct|MakeST_Player PlayerName (.Color (Utilities|Struct|BreakST_Player (Variables|Default|GetPlayer0))) (.Index (Utilities|Struct|BreakST_Player (Variables|Default|GetPlayer0))) (.isInCheckFlag (Utilities|Struct|BreakST_Player (Variables|Default|GetPlayer0))) (.HasLegalMoves (Utilities|Struct|BreakST_Player (Variables|Default|GetPlayer0))) (.MoveCount (Utilities|Struct|BreakST_Player (Variables|Default|GetPlayer0))) (.Captures (Utilities|Struct|BreakST_Player (Variables|Default|GetPlayer0))))))
    (:1
      (Variables|Default|SetPlayer1 (Utilities|Struct|MakeST_Player PlayerName (.Color (Utilities|Struct|BreakST_Player (Variables|Default|GetPlayer1))) (.Index (Utilities|Struct|BreakST_Player (Variables|Default|GetPlayer1))) (.isInCheckFlag (Utilities|Struct|BreakST_Player (Variables|Default|GetPlayer1))) (.HasLegalMoves (Utilities|Struct|BreakST_Player (Variables|Default|GetPlayer1))) (.MoveCount (Utilities|Struct|BreakST_Player (Variables|Default|GetPlayer1))) (.Captures (Utilities|Struct|BreakST_Player (Variables|Default|GetPlayer1))))))))

(fn IncrementPlayerMoveCount
  (params (PlayerIndex :type Integer))
  (switch int PlayerIndex
    (:0
      (Variables|Default|SetPlayer0 (Utilities|Struct|MakeST_Player (.Name (Utilities|Struct|BreakST_Player (Variables|Default|GetPlayer0))) (.Color (Utilities|Struct|BreakST_Player (Variables|Default|GetPlayer0))) (.Index (Utilities|Struct|BreakST_Player (Variables|Default|GetPlayer0))) (.isInCheckFlag (Utilities|Struct|BreakST_Player (Variables|Default|GetPlayer0))) (.HasLegalMoves (Utilities|Struct|BreakST_Player (Variables|Default|GetPlayer0))) (+ (.MoveCount (Utilities|Struct|BreakST_Player (Variables|Default|GetPlayer0))) 1) (.Captures (Utilities|Struct|BreakST_Player (Variables|Default|GetPlayer0))))))
    (:1
      (Variables|Default|SetPlayer1 (Utilities|Struct|MakeST_Player (.Name (Utilities|Struct|BreakST_Player (Variables|Default|GetPlayer1))) (.Color (Utilities|Struct|BreakST_Player (Variables|Default|GetPlayer1))) (.Index (Utilities|Struct|BreakST_Player (Variables|Default|GetPlayer1))) (.isInCheckFlag (Utilities|Struct|BreakST_Player (Variables|Default|GetPlayer1))) (.HasLegalMoves (Utilities|Struct|BreakST_Player (Variables|Default|GetPlayer1))) (+ (.MoveCount (Utilities|Struct|BreakST_Player (Variables|Default|GetPlayer1))) 1) (.Captures (Utilities|Struct|BreakST_Player (Variables|Default|GetPlayer1))))))))

(fn IncrementPlayerCaptureCount
  (params (PlayerIndex :type Integer))
  (switch int PlayerIndex
    (:0
      (Variables|Default|SetPlayer0 (Utilities|Struct|MakeST_Player (.Name (Utilities|Struct|BreakST_Player (Variables|Default|GetPlayer0))) (.Color (Utilities|Struct|BreakST_Player (Variables|Default|GetPlayer0))) (.Index (Utilities|Struct|BreakST_Player (Variables|Default|GetPlayer0))) (.isInCheckFlag (Utilities|Struct|BreakST_Player (Variables|Default|GetPlayer0))) (.HasLegalMoves (Utilities|Struct|BreakST_Player (Variables|Default|GetPlayer0))) (.MoveCount (Utilities|Struct|BreakST_Player (Variables|Default|GetPlayer0))) (+ (.Captures (Utilities|Struct|BreakST_Player (Variables|Default|GetPlayer0))) 1))))
    (:1
      (Variables|Default|SetPlayer1 (Utilities|Struct|MakeST_Player (.Name (Utilities|Struct|BreakST_Player (Variables|Default|GetPlayer1))) (.Color (Utilities|Struct|BreakST_Player (Variables|Default|GetPlayer1))) (.Index (Utilities|Struct|BreakST_Player (Variables|Default|GetPlayer1))) (.isInCheckFlag (Utilities|Struct|BreakST_Player (Variables|Default|GetPlayer1))) (.HasLegalMoves (Utilities|Struct|BreakST_Player (Variables|Default|GetPlayer1))) (.MoveCount (Utilities|Struct|BreakST_Player (Variables|Default|GetPlayer1))) (+ (.Captures (Utilities|Struct|BreakST_Player (Variables|Default|GetPlayer1))) 1))))))

(fn SetKinginCheckFlag
  (params (PlayerIndex :type Integer) (IsInCheck :type Boolean))
  (switch int PlayerIndex
    (:0
      (Variables|Default|SetPlayer0 (Utilities|Struct|MakeST_Player (.Name (Utilities|Struct|BreakST_Player (Variables|Default|GetPlayer0))) (.Color (Utilities|Struct|BreakST_Player (Variables|Default|GetPlayer0))) (.Index (Utilities|Struct|BreakST_Player (Variables|Default|GetPlayer0))) IsInCheck (.HasLegalMoves (Utilities|Struct|BreakST_Player (Variables|Default|GetPlayer0))) (.MoveCount (Utilities|Struct|BreakST_Player (Variables|Default|GetPlayer0))) (.Captures (Utilities|Struct|BreakST_Player (Variables|Default|GetPlayer0))))))
    (:1
      (Variables|Default|SetPlayer1 (Utilities|Struct|MakeST_Player (.Name (Utilities|Struct|BreakST_Player (Variables|Default|GetPlayer1))) (.Color (Utilities|Struct|BreakST_Player (Variables|Default|GetPlayer1))) (.Index (Utilities|Struct|BreakST_Player (Variables|Default|GetPlayer1))) IsInCheck (.HasLegalMoves (Utilities|Struct|BreakST_Player (Variables|Default|GetPlayer1))) (.MoveCount (Utilities|Struct|BreakST_Player (Variables|Default|GetPlayer1))) (.Captures (Utilities|Struct|BreakST_Player (Variables|Default|GetPlayer1))))))))

(fn SetHasLegalMovesFlag
  (params (PlayerIndex :type Integer) (HasLegalMoves :type Boolean))
  (switch int PlayerIndex
    (:0
      (Variables|Default|SetPlayer0 (Utilities|Struct|MakeST_Player (.Name (Utilities|Struct|BreakST_Player (Variables|Default|GetPlayer0))) (.Color (Utilities|Struct|BreakST_Player (Variables|Default|GetPlayer0))) (.Index (Utilities|Struct|BreakST_Player (Variables|Default|GetPlayer0))) (.isInCheckFlag (Utilities|Struct|BreakST_Player (Variables|Default|GetPlayer0))) HasLegalMoves (.MoveCount (Utilities|Struct|BreakST_Player (Variables|Default|GetPlayer0))) (.Captures (Utilities|Struct|BreakST_Player (Variables|Default|GetPlayer0))))))
    (:1
      (Variables|Default|SetPlayer1 (Utilities|Struct|MakeST_Player (.Name (Utilities|Struct|BreakST_Player (Variables|Default|GetPlayer1))) (.Color (Utilities|Struct|BreakST_Player (Variables|Default|GetPlayer1))) (.Index (Utilities|Struct|BreakST_Player (Variables|Default|GetPlayer1))) (.isInCheckFlag (Utilities|Struct|BreakST_Player (Variables|Default|GetPlayer1))) HasLegalMoves (.MoveCount (Utilities|Struct|BreakST_Player (Variables|Default|GetPlayer1))) (.Captures (Utilities|Struct|BreakST_Player (Variables|Default|GetPlayer1))))))))

(fn RotateCamera
  (params (Axis :type Float%20%28single-precision%29))
  (if (!= Axis 0.0)
    (Transformation|SetRelativeRotation (Variables|Default|GetCameraAzimuth) (Math|Rotator|MakeRotator 0.0 0.0 (+ Axis (.yaw (Variables|/Script/Engine.SceneComponent|GetRelativeRotation (Variables|Default|GetCameraAzimuth))))) false false)))