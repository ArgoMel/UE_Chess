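; King chess piece Blueprint for BattleChess that highlights the king's move options, including castling.
; ShowPossibleMoves clears highlights, then tests eight direction offsets for valid, non-friendly squares, though HighlightKingSquare sets target Y to 0, leaving YIncr unused.
; If the king is unmoved, uncastled and not in check, EvaluateCastlePath walks both ways along Y over empty squares.
; An unmoved friendly rook at the edge highlights a two-square castle move.
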(fn ConstructionScript
  (|CallParentFunction))

(fn ShowPossibleMoves
  (Utilities|FlowControl|Sequence
    (:then_0
      (Class|GMChess|UnhighlightSquares (Variables|Default|GetGameModeRef))
      (Variables|Default|SetKindCanCastle false)
      (Variables|Default|SetKingIsCastling false))
    (:then_1
      (CallFunction|HighlightKingSquare 1)
      (CallFunction|HighlightKingSquare 1 1)
      (CallFunction|HighlightKingSquare 1 -1))
    (:then_2
      (CallFunction|HighlightKingSquare -1)
      (CallFunction|HighlightKingSquare -1 1)
      (CallFunction|HighlightKingSquare -1 -1))
    (:then_3
      (CallFunction|HighlightKingSquare 0 1)
      (CallFunction|HighlightKingSquare 0 -1))
    (:then_4
      (CallFunction|EvaluateCastleSquares)
      (return (Variables|Default|GetIsKing)))))

(fn HighlightKingSquare
  (params (XIncr :type Integer) (YIncr :type Integer))
  (LocalVariables|SetTempX (+ (Variables|Default|GetX) XIncr))
  (LocalVariables|SetTempY 0)
  (if (CallFunction|IsValidMoveforKing (LocalVariables|GetTempX) (LocalVariables|GetTempY))
    (Class|ChessPiece|HighlightPotentialSquare (LocalVariables|GetTempX) (LocalVariables|GetTempY) (Variables|Default|GetColor))))

(fn IsValidMoveforKing
  (params (X :type Integer) (Y :type Integer))
  (bind _gamemoderef (Variables|Default|GetGameModeRef))
  (bind _color (Variables|Default|GetColor))
  (bind (_isoccupied _isoccupiedbyfriend _isvalidsquare) (Class|GMChess|GetOccupant _gamemoderef X Y _color))
  (return (and _isvalidsquare (not _isoccupiedbyfriend))))

(fn EvaluateCastlePath
  (params (YIncr :type Integer))
  (LocalVariables|SetIsPositive (> YIncr 0))
  (LocalVariables|SetTempY (Variables|Default|GetY))
  (LocalVariables|SetCanContinue true)
  (while (LocalVariables|GetCanContinue)
    (LocalVariables|SetTempY (+ (LocalVariables|GetTempY) YIncr))
    (if (and (< (LocalVariables|GetTempY) 8) (> (LocalVariables|GetTempY) 1))
      (LocalVariables|SetCanContinue (not (.IsOccupied (Class|GMChess|GetOccupant (Variables|Default|GetGameModeRef) (Variables|Default|GetX) (LocalVariables|GetTempY) (Variables|Default|GetColor)))))
      (elif (and (.IsOccupiedByFriend (Class|GMChess|GetOccupant (Variables|Default|GetGameModeRef) (Variables|Default|GetX) (LocalVariables|GetTempY) (Variables|Default|GetColor))) (.bSuccess (Utilities|Casting|CastToBP_Rook (.ReturnValue (Class|GMChess|GetOccupant (Variables|Default|GetGameModeRef) (Variables|Default|GetX) (LocalVariables|GetTempY) (Variables|Default|GetColor))))))
        (if (Variables|/Script/BattleChess.ChessPiece|GetIsInitialMove (.AsBP%20Rook (Utilities|Casting|CastToBP_Rook (.ReturnValue (Class|GMChess|GetOccupant (Variables|Default|GetGameModeRef) (Variables|Default|GetX) (LocalVariables|GetTempY) (Variables|Default|GetColor))))))
          (CallFunction|HighlightCastleSquares (LocalVariables|GetIsPositive))
          (LocalVariables|SetCanContinue false :!label _label))
        (else
          (goto _label))))))

(fn HighlightCastleSquares
  (params (IsPositive :type Boolean))
  (bind _y (Variables|Default|GetY))
  (bind _returnvalue (+ _y -2))
  (if IsPositive
    (bind _output_get (LocalVariables|SetTempY (+ _y 2)))
    (Class|ChessPiece|HighlightPotentialSquare (Variables|Default|GetX) _output_get (Variables|Default|GetColor))
    (Variables|Default|SetKingCanCastle true)
    (else
      (LocalVariables|SetTempY _returnvalue)
      (Class|ChessPiece|HighlightPotentialSquare (Variables|Default|GetX) _returnvalue (Variables|Default|GetColor))
      (Variables|Default|SetKingCanCastle true))))

(fn EvaluateCastleSquares
  (Variables|Default|SetKindCanCastle false)
  (if (not (Variables|Default|GetKingHasCastled))
    (if (Variables|Default|GetIsInitialMove)
      (if (not (Class|GMChess|IsActiveKingCheckStatus (Variables|Default|GetGameModeRef)))
        (Utilities|FlowControl|Sequence
          (:then_0
            (CallFunction|EvaluateCastlePath 1))
          (:then_1
            (CallFunction|EvaluateCastlePath -1)))
        (else
          (Variables|Default|SetKingCanCastle false :!label _label)))
      (else
        (goto _label)))
    (else
      (goto _label))))