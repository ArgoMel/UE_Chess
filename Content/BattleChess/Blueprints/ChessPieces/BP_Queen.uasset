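; BP_Queen is the queen chess piece Blueprint in BattleChess, defining which squares it can move to.
; ShowPossibleMoves clears existing highlights through the game mode, then highlights diagonal, horizontal and vertical squares for the piece's Color using inherited helpers.
; It returns IsKing, and the construction script only calls the parent's.
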(fn ConstructionScript
  (|CallParentFunction))

(fn ShowPossibleMoves
  (bind _color (Variables|Default|GetColor))
  (Utilities|FlowControl|Sequence
    (:then_0
      (Class|GMChess|UnhighlightSquares (Variables|Default|GetGameModeRef)))
    (:then_1
      (Class|ChessPiece|HighlightDiagonalSquares _color)
      (Class|ChessPiece|HighlightHorizontalSquares _color)
      (Class|ChessPiece|HighlightVerticalSquares _color))
    (:then_2
      (return (Variables|Default|GetIsKing)))))